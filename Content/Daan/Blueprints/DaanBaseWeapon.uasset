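; Base weapon Blueprint that handles raising and lowering a weapon, with an empty Attack function.
; RaiseWeapon and LowerWeapon toggle IsActive, print a debug message and call the Move event with a fixed vertical vector.
; Move passes that vector to MoveComponentTo as the root's target relative location.
; Init copies active and picked-up state from WeaponInfo, raising the weapon first if it is active.
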(event Custom|Move
  (params (MoveVector :type Vector))
  (Components|MoveComponentTo (Variables|Default|GetDefaultSceneRoot) MoveVector "0, 0, 0" false false 0.2 false))

(event EventBeginPlay)

(event Collision|EventActorBeginOverlap
  (params (OtherActor :type Actor%20Object%20Reference)))

(event EventTick
  (params (DeltaSeconds :type Float%20%28single-precision%29)))

(fn ConstructionScript)

(fn Attack)

(fn LowerWeapon
  (if (Variables|Default|GetIsActive)
    (Development|PrintString "Lower weapon")
    (Variables|Default|SetIsActive false)
    (CallFunction|Move "0, 0,-100.000000")))

(fn RaiseWeapon
  (if (not (Variables|Default|GetIsActive))
    (Development|PrintString "Raise weapon" true true "(R=1.000000,G=0.124931,B=0.000000,A=1.000000)")
    (Variables|Default|SetIsActive true)
    (CallFunction|Move "0, 0,100.000000")))

(fn Init
  (params (WeaponInfo :type Daan%20Weapon%20Info%20Structure))
  (bind (_isactive _havepickedup) (Utilities|Struct|BreakDaanWeaponInfo WeaponInfo))
  (if _isactive
    (CallFunction|RaiseWeapon)
    (Variables|Default|SetIsActive _isactive)
    (Variables|Default|SetHavePickedUp _havepickedup)
    (else
      (Variables|Default|SetIsActive _isactive)
      (Variables|Default|SetHavePickedUp _havepickedup))))