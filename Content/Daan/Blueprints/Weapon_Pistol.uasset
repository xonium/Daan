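; Pistol weapon Blueprint that fires hitscan shots from the first-person camera, ignoring the player character.
; Each shot line-traces forward, draws a persistent debug line and only prints the hit actor's name, with no damage applied.
; StartAttack sets a looping timer at AttackSpeed for automatic repeat fire while attacking.
; StopAttack clears that timer and blocks firing for one AttackSpeed interval, while LowerWeapon also cancels repeat fire.
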(event EventBeginPlay
  (|CallParentFunction)
  (Utilities|Array|Add (Variables|Default|GetActorsToIgnore) (Game|GetPlayerCharacter 0)))

(event Collision|EventActorBeginOverlap
  (params (OtherActor :type Actor%20Object%20Reference))
  (|CallParentFunction OtherActor) ; This node is disabled and will not be called.\nDrag off pins to build functionality.
)

(event EventTick
  (params (DeltaSeconds :type Float%20%28single-precision%29))
  (|CallParentFunction DeltaSeconds) ; This node is disabled and will not be called.\nDrag off pins to build functionality.
)

(event EventStartAttack
  (if (Variables|Default|GetCanAttack)
    (bind _asdaan_player_character (Utilities|Casting|CastToDaanPlayerCharacter (Game|GetPlayerCharacter 0)))
    (bind _outhit (Collision|LineTraceForObjects (Transformation|GetWorldLocation (Variables|/Game/Daan/Blueprints/DaanPlayerCharacter.DaanPlayerCharacter_C|GetFirstPersonCamera _asdaan_player_character)) (+ (* (Math|Vector|GetForwardVector (Variables|/Game/Daan/Blueprints/DaanPlayerCharacter.DaanPlayerCharacter_C|GetFirstPersonCamera _asdaan_player_character)) 1e+04) (Transformation|GetWorldLocation (Variables|/Game/Daan/Blueprints/DaanPlayerCharacter.DaanPlayerCharacter_C|GetFirstPersonCamera _asdaan_player_character))) (Variables|Default|GetAllObjects) false (Variables|Default|GetActorsToIgnore) "Persistent"))
    (Development|PrintString (Utilities|GetDisplayName (.HitActor (Collision|BreakHitResult _outhit))))
    (bind _returnvalue (Utilities|Time|SetTimerbyEvent (delegate EventStartAttack) (Variables|Default|GetAttackSpeed) true))
    (Variables|Default|SetAttack_Timer_Handle _returnvalue)))

(event EventStopAttack
  (if (Variables|Default|GetCanAttack)
    (Variables|Default|SetCanAttack false)
    (Utilities|Time|ClearandInvalidateTimerbyHandle (Variables|Default|GetAttack_Timer_Handle))
    (bind _returnvalue (Utilities|Time|SetTimerbyEvent (delegate EventSetCanAttackAgain) (Variables|Default|GetAttackSpeed)))))

(event EventLowerWeapon
  (|CallParentFunction)
  (Utilities|Time|ClearandInvalidateTimerbyHandle (Variables|Default|GetAttack_Timer_Handle)))

(event EventSetCanAttackAgain
  (Variables|Default|SetCanAttack true)
  (Utilities|Time|ClearandInvalidateTimerbyHandle (stale EventStopAttack _returnvalue)))

(fn ConstructionScript
  (|CallParentFunction))